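; NPC Blueprint that sketches a state machine for moving to a target and using workstations.
; A once-per-second delta accumulator is meant to call UpdateState, then act by state: AI Move To, or a distance check against the workstation's animation origin.
; UpdateState switches workstation states to Move to Target when the target is not an NPCWorkstation.
; The logic is unfinished: Tick is unwired and the distance check leads nowhere.
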(event `self.ReceiveTick`
  (params (DeltaSeconds :type "Float (single-precision)"))
  ;[1 1 1] Once Per Second
)

(fn `UpdateState`
  (params (NPCState :type "ENPCStateEnum Enum (by ref)" :default "VE_Idle") (TargetActor :type "Actor Object Reference"))
  (switch `ENPCStateEnum` NPCState
    (:`VE_WorkstationBegin`
      _)
    (:`VE_WorkstationLoop`
      _)
    (:`VE_WorkstationExit`
      _))
  ;[1 1 1] If we are in a workstation state and our target actor isn't a workstation, enter the MoveToTarget State
  (if (not (== (`GameplayStatics.GetObjectClass` TargetActor) "/Script/SlaveVRExperience.NPCWorkstation"))
    (set `self.NPCState` "VE_MoveToTarget")))

(fn `UserConstructionScript`)