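; NPC character Blueprint that walks toward a TargetActor using AI navigation.
; BeginPlay sets the movement component's max walk speed from the NPCSpeedMax variable.
; Tick accumulates delta time and reissues AIMoveTo about once per second, carrying over the remainder, rather than every frame.
; The Path function and construction script are empty.
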(event `self.ReceiveTick`
  (params (DeltaSeconds :type "Float (single-precision)"))
  ;[1 1 1] Once Per Second
  (bind _output_get (set `self.currentDelta` (+ DeltaSeconds (`self.currentDelta`))))
  (if (>= _output_get 1.0)
    (`|ExecutionSequence`
      (:`then_0`
        (set `self.currentDelta` (- (`self.currentDelta`) 1.0)))
      (:`then_1`
        ;[1 1 1] Path To Destination
        (`|AIMoveTo` self (0.0 0.0 0.0) (`self.TargetActor`))))))

(event `self.ReceiveBeginPlay`
  ;[1 1 1] Set Walkspeed From Interface
  (set `CharacterMovementComponent.MaxWalkSpeed` (`self.NPC Speed Max`) (`self.CharacterMovement`)))

(fn `Path`)

(fn `UserConstructionScript`)